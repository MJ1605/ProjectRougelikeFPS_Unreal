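; Base enemy Blueprint that tracks health and rewards the player with XP and coins when it is destroyed.
; On BeginPlay it raises itself by a height offset, binds damage handling, fills health to max and caches the player controller.
; Damage reduces health and destroys the actor at zero.
; EndPlay with reason Destroyed passes the drops to the controller's death handler and fires an enemy despawn dispatcher.
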(event EventBeginPlay
  (bind _capsulecomponent (Variables|Collision|GetCapsuleComponent))
  (bind _returnvalue (Transformation|GetWorldLocation _capsulecomponent))
  (bind (_x _y _z) (Class|KismetMathLibrary|BreakVector3f _returnvalue))
  (Transformation|SetWorldLocation _capsulecomponent (Math|Vector|MakeVector _x _y (+ _z (Variables|Default|GetfHeight))) false false)
  (EventDispatchers|AssignOnTakeAnyDamage (EventDispatchers|CreateEvent :!event TakeDamage))
  (Variables|Default|SetfHealth (Variables|Default|GetMaxHealth))
  (bind _asbp_player_controller (Utilities|Casting|CastToBP_PlayerController (Game|GetPlayerController 0)))
  (Variables|Default|SetPlayerControllerRef _asbp_player_controller))

(event EventEndPlay
  (params (EndPlayReason :type EEndPlayReason%20Enum :default "Destroyed"))
  (switch Utilities|FlowControl|Switch|SwitchonEEndPlayReason EndPlayReason
    (:Destroyed
      (Default|EnemyDeathHandler (Variables|Default|GetPlayerControllerRef) (Variables|Default|GetXPDrop) (Variables|Default|GetCoinsDrop))
      (Default|CallEveEnemyDespawn))))

(fn ConstructionScript)

(fn TakeDamage
  (params (DamagedActor :type Actor%20Object%20Reference) (Damage :type Float%20%28single-precision%29) (DamageType :type Damage%20Type%20Object%20Reference) (InstigatedBy :type Controller%20Object%20Reference) (DamageCauser :type Actor%20Object%20Reference))
  (bind _output_get (Variables|Default|SetfHealth (- (Variables|Default|GetfHealth) Damage)))
  (if (<= _output_get 0.0)
    (Actor|DestroyActor)))