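; Basic crawler enemy character that chases the first-person player and deals damage at close range.
; Tick counts down an attack cooldown, then compares squared capsule distance to either attack or issue AIMoveTo toward the player.
; Incoming damage reduces health and destroys the actor at zero.
; An ApplyForce event lets the crawler be pushed with a mass-independent velocity impulse.
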(event Custom|OnTakeAnyDamage_Event
  (params (DamagedActor :type Actor%20Object%20Reference) (Damage :type Float%20%28single-precision%29) (DamageType :type Damage%20Type%20Object%20Reference) (InstigatedBy :type Controller%20Object%20Reference) (DamageCauser :type Actor%20Object%20Reference))
  (bind _output_get (Variables|Default|SetCurrentHealth (- (Variables|Default|GetCurrentHealth) Damage)))
  (if (<= _output_get 0.0)
    (Actor|DestroyActor)))

(event EventBeginPlay
  (Variables|Default|SetCurrentHealth (Variables|Default|GetMaxHealth))
  (bind _asbp_first_person_character (Utilities|Casting|CastToBP_FirstPersonCharacter (Game|Player|GetPlayerPawn 0)))
  (Variables|Default|SetPlayerPawnRef _asbp_first_person_character)
  (EventDispatchers|BindEventtoOnTakeAnyDamage (delegate Custom|OnTakeAnyDamage_Event)))

(event EventTick
  (params (DeltaSeconds :type Float%20%28single-precision%29))
  (Utilities|ProcessDamagedt DeltaSeconds
    (:out
      (if (<= (Math|Vector|VectorLengthSquared (- (Transformation|GetWorldLocation (Variables|/Script/Engine.Character|GetCapsuleComponent (Variables|Default|GetPlayerPawnRef))) (Transformation|GetWorldLocation (Variables|Collision|GetCapsuleComponent)))) (Math|Float|Square (Variables|Default|GetDamageDistance)))
        (if (== (Variables|Default|GetAttackdt) 0.0)
          (Game|Damage|ApplyDamage (Variables|Default|GetPlayerPawnRef) (Variables|Default|GetDamage) 0 0)
          (Variables|Default|SetAttackdt (Variables|Default|GetTimeBetweenAttacks)))
        (else
          (AI|AIMoveTo self "0, 0, 0" (Variables|Default|GetPlayerPawnRef) 5.0 false))))))

(event EventApplyForce
  (params (Force :type Vector :default "0, 0, 0"))
  (Physics|AddImpulse (Variables|Character|GetCharacterMovement) Force true))

(fn ConstructionScript)