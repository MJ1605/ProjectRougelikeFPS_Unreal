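; Gun-wielding crawler enemy that chases the first-person player and fires bullets at them.
; Each tick counts down an attack cooldown, then spawns a BP_CrawlerBullet aimed at the player's capsule and passes it the damage, regardless of distance.
; Movement re-issues AIMoveTo toward the player every tick, switching the target to itself to hold position once within DamageDist, compared using squared distance.
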(event EventBeginPlay
  (|CallParentFunction)
  (bind _asbp_first_person_character (Utilities|Casting|CastToBP_FirstPersonCharacter (Game|Player|GetPlayerPawn 0)))
  (Variables|Default|SetPlayerPawnRef _asbp_first_person_character))

(event EventEndPlay
  (params (EndPlayReason :type EEndPlayReason%20Enum :default "Destroyed"))
  (|CallParentFunction EndPlayReason))

(event EventTick
  (params (DeltaSeconds :type Float%20%28single-precision%29))
  (bind _self self)
  (bind _capsulecomponent (Variables|Default|GetCapsuleComponent))
  (bind _playerpawnref (Variables|Default|GetPlayerPawnRef))
  (bind _returnvalue (Transformation|GetWorldLocation _capsulecomponent))
  (bind _capsulecomponent_2 (Variables|/Script/Engine.Character|GetCapsuleComponent _playerpawnref))
  (bind _returnvalue_2 (Transformation|GetWorldLocation _capsulecomponent_2))
  (bind _returnvalue_3 (- _returnvalue_2 _returnvalue))
  (Utilities|UpdateAttackdt DeltaSeconds
    (:Out
      (if (== (Variables|Default|GetAttackdt) 0.0)
        (bind _returnvalue_4 (Game|SpawnActorfromClass "/Game/Enemies/CrawlerWithGun/BP_CrawlerBullet.BP_CrawlerBullet_C" (Math|Transform|MakeTransform (Transformation|GetWorldLocation (Variables|Default|GetBulletSpawn)) (Math|Rotator|MakeRotfromX (Math|Vector|Normalize _returnvalue_3))) "Undefined" 0 self))
        (Variables|Default|SetAttackdt (Variables|Default|GetTimebetweenAttack))
        (Variables|/Game/Enemies/CrawlerWithGun/BP_CrawlerBullet.BP_CrawlerBullet_C|SetDamage _returnvalue_4 (Variables|Default|GetDamage)))
      ;[1 1 1] Movement
      (if (<= (Math|Vector|VectorLengthSquared _returnvalue_3) (Math|Float|Square (Variables|Default|GetDamageDist)))
        (AI|AIMoveTo _self "0, 0, 0" _self 5.0 false)
        (else
          (AI|AIMoveTo self "0, 0, 0" (Variables|Default|GetPlayerPawnRef) 5.0 false))))))

(fn ConstructionScript)