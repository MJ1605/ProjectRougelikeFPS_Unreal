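; Test enemy that chases the player once PawnSensing sees a pawn and destroys itself when health runs out.
; Damage comes from AnyDamage or a player-controller event that damages all enemies, and feeds a debug health bar widget.
; GameManager events toggle that bar's visibility and world or screen space, with Tick rotating it toward the camera in world space.
; The seen flag is never cleared here.
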(event OnSeePawn(PawnSensing)
  (params (Pawn :type Pawn%20Object%20Reference))
  (Variables|Default|SetbIsSeeingPlayer true)
  (CallFunction|FollowPlayer))

(event Custom|Follow%20Player
  (if (Variables|Default|GetbIsSeeingPlayer)
    (AI|AIMoveTo self "0, 0, 0" (Game|GetPlayerCharacter 0) 5.0 false)))

(event Custom|Toggle%20HP%20Bar
  (params (HPBar%20Status :type Boolean))
  (Debug|ToggleHPBar HPBar%20Status))

(event Custom|Toggle%20HP%20Render%20Space
  (params (IsWorld :type Boolean))
  (Debug|ToggleHPBarRenderSpace IsWorld))

(event Custom|Universal%20Damage%20Taking
  (CallFunction|TakeDamage 25.0))

(event EventBeginPlay
  (Variables|Default|SetfMaxHealth (Variables|Default|GetfHealth))
  (bind _asbp_player_controller (Utilities|Casting|CastToBP_PlayerController (Game|GetPlayerController 0)))
  (EventDispatchers|BindEventtoDealDamagetoAllEnemies _asbp_player_controller (delegate Custom|Universal%20Damage%20Taking))
  (bind _asgame_manager (Utilities|Casting|CastToGameManager (Game|GetGameInstance)))
  (bind _output_get (Variables|Default|SetGame%20Manager _asgame_manager))
  (Debug|ToggleHPBar (Variables|/Game/GameManager.GameManager_C|GetbEnemyHPBar _output_get))
  (EventDispatchers|BindEventtoToggleEnemyHPBar _asgame_manager (delegate Custom|Toggle%20HP%20Bar))
  (EventDispatchers|BindEventtoToggleEHPBarRenderSpace _asgame_manager (delegate Custom|Toggle%20HP%20Render%20Space))
  (bind _aswb_enemy_health (Utilities|Casting|CastToWB_EnemyHealth (UserInterface|GetWidget (Variables|Default|GetDebug%20HealthBar))))
  (bind _output_get_2 (Variables|Default|SetHealthBar _aswb_enemy_health))
  (Default|SetMaxHealth _output_get_2 (Variables|Default|GetfMaxHealth) (Variables|Default|GetfMaxHealth)))

(event Game|Damage|EventAnyDamage
  (params (Damage :type Float%20%28single-precision%29) (DamageType :type Damage%20Type%20Object%20Reference) (InstigatedBy :type Controller%20Object%20Reference) (DamageCauser :type Actor%20Object%20Reference))
  ;[1 1 1] Handle Damage Taking
  (CallFunction|TakeDamage Damage))

(event EventTick
  (params (DeltaSeconds :type Float%20%28single-precision%29))
  (Debug|HPBarFaceCamera))

(fn ConstructionScript)

(fn TakeDamage
  (params (Damage :type Float%20%28double-precision%29))
  (bind _output_get (Variables|Default|SetfHealth (- (Variables|Default|GetfHealth) Damage)))
  (if (> _output_get (Variables|Default|GetfMaxHealth))
    (Variables|Default|SetfHealth (Variables|Default|GetfMaxHealth))
    (elif (<= (Variables|Default|GetfHealth) 0.0)
      (Actor|DestroyActor)))
  (Default|UpdateHealth (Variables|Default|GetHealthBar) (Variables|Default|GetfHealth)))

(fn ToggleHPBar
  (params (HP%20Status :type Boolean))
  (Rendering|SetVisibility (Variables|Default|GetDebug%20HealthBar) HP%20Status true))

(fn ToggleHPBarRenderSpace
  (params (IsWorld :type Boolean))
  (Class|WidgetComponent|SetWidgetSpace (Variables|Default|GetDebug%20HealthBar) (select IsWorld "World" "Screen")))

(fn HPBarFaceCamera
  ;[1 1 1] Make the debug health bar face the camera
  (if (Variables|/Game/GameManager.GameManager_C|GetbEnemyHPBarIsWorld (Variables|Default|GetGame%20Manager))
    (Transformation|SetWorldRotation (Variables|Default|GetDebug%20HealthBar) (Math|Rotator|FindLookatRotation (Transformation|GetWorldLocation (Variables|Default|GetDebug%20HealthBar)) (Transformation|GetActorLocation (Game|GetPlayerCameraManager 0))) false false)))