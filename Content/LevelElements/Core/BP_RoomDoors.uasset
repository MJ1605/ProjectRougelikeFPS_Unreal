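; Room door level element that opens and closes by hiding or showing its Door component.
; ToggleDoorState flips IsDoorOpened, then calls ToggleDoorAttributes, which also runs on BeginPlay to apply the initial state.
; When open, the door and its children are invisible and Door collision is disabled; when closed, it is visible with query and physics collision, with no animation.
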(event Custom|Toggle%20Door%20State
  (Variables|Default|SetIsDoorOpened (not (Variables|Default|GetIsDoorOpened)))
  (CallFunction|ToggleDoorAttributes))

(event EventBeginPlay
  (CallFunction|ToggleDoorAttributes))

(fn ConstructionScript)

(fn ToggleDoorAttributes
  (bind _isdooropened (Variables|Default|GetIsDoorOpened))
  (bind _door (Variables|Default|GetDoor))
  (Rendering|SetVisibility _door (not _isdooropened) true)
  (Collision|SetCollisionEnabled _door (select _isdooropened "NoCollision" "QueryAndPhysics")))