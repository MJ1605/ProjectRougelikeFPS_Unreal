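; BP_Trap is a damaging level element that applies environmental damage once to any actor that begins overlapping its Trigger component.
; Each overlap also switches the trigger material's BaseColor to the triggered color, resets a countdown and increments an in-range counter.
; Tick runs the countdown only while nothing is overlapping, restoring the normal color when it expires.
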(event OnComponentBeginOverlap(Trigger)
  (params (OverlappedComponent :type Primitive%20Component%20Object%20Reference) (OtherActor :type Actor%20Object%20Reference) (OtherComp :type Primitive%20Component%20Object%20Reference) (OtherBodyIndex :type Integer) (bFromSweep :type Boolean) (SweepResult :type Hit%20Result%20Structure%20%28by%20ref%29))
  (Game|Damage|ApplyDamage OtherActor (Variables|Default|GetTrap%20Damage) 0 self "/Engine/EngineDamageTypes/DmgTypeBP_Environmental.DmgTypeBP_Environmental_C")
  (Rendering|Material|SetVectorParameterValueonMaterials (Variables|Default|GetTrigger) "BaseColor" (Math|Conversions|ToVector(LinearColor) (Variables|Default|GetTriggeredColor)))
  (Variables|Default|SetTriggerdt (Variables|Default|GetTriggeredTime))
  (Math|Integer|IncrementInt (Variables|Default|GetNumInRange)))

(event OnComponentEndOverlap(Trigger)
  (params (OverlappedComponent :type Primitive%20Component%20Object%20Reference) (OtherActor :type Actor%20Object%20Reference) (OtherComp :type Primitive%20Component%20Object%20Reference) (OtherBodyIndex :type Integer))
  (Math|Integer|DecrementInt (Variables|Default|GetNumInRange)))

(event EventTick
  (params (DeltaSeconds :type Float%20%28single-precision%29))
  (if (== (Variables|Default|GetNumInRange) 0)
    (if (> (Variables|Default|GetTriggerdt) 0.0)
      (bind _output_get (Variables|Default|SetTriggerdt (- (Variables|Default|GetTriggerdt) DeltaSeconds)))
      (if (<= _output_get 0.0)
        (Rendering|Material|SetVectorParameterValueonMaterials (Variables|Default|GetTrigger) "BaseColor" (Math|Conversions|ToVector(LinearColor) (Variables|Default|GetNormalColor)))
        (Variables|Default|SetTriggerdt 0.0)))))

(fn ConstructionScript)