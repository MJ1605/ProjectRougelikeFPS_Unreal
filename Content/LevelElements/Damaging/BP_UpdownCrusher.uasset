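; BP_UpdownCrusher is a damaging level hazard that repeatedly slams its Cube down and raises it again.
; Tick runs a three-state machine: wait on a timer, fall with per-frame accumulated velocity, then rise at constant speed past the original height.
; Only a Hurtbox overlap ends the fall, applying environmental damage to whatever it hit and starting the return.
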(event OnComponentBeginOverlap(hurtbox)
  (params (OverlappedComponent :type Primitive%20Component%20Object%20Reference) (OtherActor :type Actor%20Object%20Reference) (OtherComp :type Primitive%20Component%20Object%20Reference) (OtherBodyIndex :type Integer) (bFromSweep :type Boolean) (SweepResult :type Hit%20Result%20Structure%20%28by%20ref%29))
  (switch Utilities|FlowControl|Switch|SwitchonCrusherStates (Variables|Default|GetState)
    (:NewEnumerator1
      (Variables|Default|SetState "NewEnumerator2")
      (Game|Damage|ApplyDamage OtherActor (Variables|Default|GetDamage) 0 self "/Engine/EngineDamageTypes/DmgTypeBP_Environmental.DmgTypeBP_Environmental_C"))))

(event EventTick
  (params (DeltaSeconds :type Float%20%28single-precision%29))
  (bind _cube (Variables|Default|GetCube))
  (bind _returnspeed (Variables|Default|GetReturnSpeed))
  (bind _cube_2 (Variables|Default|GetCube))
  (bind _returnvalue (* _returnspeed DeltaSeconds))
  (bind _relativelocation (Variables|/Script/Engine.SceneComponent|GetRelativeLocation _cube))
  (bind _relativelocation_2 (Variables|/Script/Engine.SceneComponent|GetRelativeLocation _cube_2))
  (bind (_x _y _z) (Class|KismetMathLibrary|BreakVector3f _relativelocation_2))
  (bind (_x_2 _y_2 _z_2) (Class|KismetMathLibrary|BreakVector3f _relativelocation))
  (bind _returnvalue_2 (+ _z _returnvalue))
  (switch Utilities|FlowControl|Switch|SwitchonCrusherStates (Variables|Default|GetState)
    (:NewEnumerator0
      (bind _output_get (Variables|Default|SetWaitdt (- (Variables|Default|GetWaitdt) DeltaSeconds)))
      (if (<= _output_get 0.0)
        (Variables|Default|SetState "NewEnumerator1")
        (Variables|Default|SetVelocity 0.0)))
    (:NewEnumerator1
      (bind _output_get_2 (Variables|Default|SetVelocity (+ (Variables|Default|GetCrushAceleration) (Variables|Default|GetVelocity))))
      (Transformation|SetRelativeLocation _cube (Math|Vector|MakeVector _x_2 _y_2 (- _z_2 (* _output_get_2 DeltaSeconds))) false false))
    (:NewEnumerator2
      (Transformation|SetRelativeLocation _cube_2 (Math|Vector|MakeVector _x _y _returnvalue_2) false false)
      (if (> _returnvalue_2 (.Z (Class|KismetMathLibrary|BreakVector3f (Variables|Default|GetOriginalPosition))))
        (Variables|Default|SetState "NewEnumerator0")
        (Variables|Default|SetWaitdt (Variables|Default|GetTimeBetweenCrush))))))

(event EventBeginPlay
  (Variables|Default|SetWaitdt (Variables|Default|GetTimeBetweenCrush))
  (Variables|Default|SetOriginalPosition (Variables|/Script/Engine.SceneComponent|GetRelativeLocation (Variables|Default|GetCube))))

(fn ConstructionScript)