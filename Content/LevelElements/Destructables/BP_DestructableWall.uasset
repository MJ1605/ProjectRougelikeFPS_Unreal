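; BP_DestructableWall is a destructible wall level element that takes damage and removes itself when its health runs out.
; On BeginPlay it sets Health from StartingHealth and binds to its own OnTakeAnyDamage.
; Each hit lowers Health, then either destroys the actor or tints the Cube mesh through its Color material parameter, blending from NormalColor toward DamagedColor by remaining health ratio.
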(event Custom|OnTakeAnyDamage_Event
  (params (DamagedActor :type Actor%20Object%20Reference) (Damage :type Float%20%28single-precision%29) (DamageType :type Damage%20Type%20Object%20Reference) (InstigatedBy :type Controller%20Object%20Reference) (DamageCauser :type Actor%20Object%20Reference))
  (bind _output_get (Variables|Default|SetHealth (- (Variables|Default|GetHealth) Damage)))
  (if (<= _output_get 0.0)
    (Actor|DestroyActor)
    (else
      (Rendering|Material|SetVectorParameterValueonMaterials (Variables|Default|GetCube) "Color" (Math|Conversions|ToVector(LinearColor) (Math|Color|Lerp(LinearColor) (Variables|Default|GetDamagedColor) (Variables|Default|GetNormalColor) (/ (Variables|Default|GetHealth) (Variables|Default|GetStartingHealth))))))))

(event EventBeginPlay
  (EventDispatchers|BindEventtoOnTakeAnyDamage (delegate Custom|OnTakeAnyDamage_Event))
  (Variables|Default|SetHealth (Variables|Default|GetStartingHealth)))

(fn ConstructionScript)