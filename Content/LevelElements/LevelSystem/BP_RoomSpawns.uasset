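; Room encounter actor that runs random waves of enemies and toggles the entry and exit doors around the fight.
; BeginPlay rolls the wave count, caches child spawn-point transforms and disables spawning if enemies or points are missing.
; The player's first trigger overlap starts waves of random enemies; their despawn events count down to the next wave or exit.
; UsedSpawnPoints is checked but never filled here, so spawn points can repeat.
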(event OnComponentBeginOverlap(EnterRoomTrigger)
  (params (OverlappedComponent :type Primitive%20Component%20Object%20Reference) (OtherActor :type Actor%20Object%20Reference) (OtherComp :type Primitive%20Component%20Object%20Reference) (OtherBodyIndex :type Integer) (bFromSweep :type Boolean) (SweepResult :type Hit%20Result%20Structure%20%28by%20ref%29))
  (if (not (Variables|Default|GetbIsStarted))
    (Utilities|Casting|CastToBP_FirstPersonCharacter OtherActor)
    (Variables|Default|SetbIsStarted true)
    (Default|ToggleDoorState (Variables|Default|GetEntryDoor))
    (CallFunction|SpawnWave)))

(event Custom|Spawn%20Wave
  (if (not (Variables|Default|GetIsDisabled))
    (for _index (range 0 (- (+ (Math|Random|RandomInteger (- (Variables|Default|GetMaxSpawnsPerWave) (Variables|Default|GetMinSpawnsPerWave))) (Variables|Default|GetMinSpawnsPerWave)) 1))
      (Math|Integer|IncrementInt (Variables|Default|GetTotalEnemiesAlive)
        (:%20%20
          (bind _output_get (Variables|Default|SetLastSpawnPoint (Utilities|Array|Get(acopy) (Variables|Default|GetSpawnPoints) (Math|Random|RandomInteger (Utilities|Array|Length (Variables|Default|GetSpawnPoints))))))
          (if (Utilities|Array|ContainsItem (Variables|Default|GetUsedSpawnPoints) _output_get) :!label _label
            (if true
              (goto _label)
              (else
                (goto _label)))
            (else
              (bind _returnvalue (Game|SpawnActorfromClass (Utilities|Array|Get(acopy) (Variables|Default|GetEnemies) (Math|Random|RandomInteger (Utilities|Array|Length (Variables|Default|GetEnemies)))) (Variables|Default|GetLastSpawnPoint) "AdjustIfPossibleButAlwaysSpawn" 0 0))
              (EventDispatchers|AssignEveEnemyDespawn _returnvalue (delegate Custom|Eve_EnemyDespawn_Event)))))))))

(event Custom|Eve_EnemyDespawn_Event
  (bind _result (Math|Integer|DecrementInt (Variables|Default|GetTotalEnemiesAlive))
    (:%20%20
      (if (<= _result 0) ; Check if there is any enemies left alive
        (bind _result_2 (Math|Integer|DecrementInt (Variables|Default|GetWavesRemaining))
          (:%20%20
            (if (<= _result_2 0) ; Check if there is more waves left
              (Development|PrintString "Open end door")
              (for _array_element (Variables|Default|GetExitDoor)
                (Default|ToggleDoorState _array_element))
              (else
                (CallFunction|SpawnWave) ; Spawn the next wave if there is still more waves
              ))))))))

(event EventBeginPlay
  (bind _spawnlocations (Variables|Default|GetSpawnLocations))
  (bind _returnvalue (Class|SceneComponent|GetNumChildrenComponents _spawnlocations))
  (bind _output_get (Variables|Default|SetWavesRemaining (+ (Math|Random|RandomInteger (Variables|Default|GetMaxWaves)) 1))) ; Generate the number of waves for the room
  ;[1 1 1] Precautionary Checks
  (Development|PrintString (Utilities|String|BuildString(Integer) "" "Total Waves:" _output_get))
  (if (!= (Utilities|Array|Length (Variables|Default|GetEnemies)) 0)
    (if (!= (Class|SceneComponent|GetNumChildrenComponents (Variables|Default|GetSpawnLocations)) 0)
      ;;[1 1 1] Make sure that we dont spawn more than the spawn points avaliable
      (if (> (Variables|Default|GetMaxSpawnsPerWave) _returnvalue)
        (Variables|Default|SetMaxSpawnsPerWave _returnvalue))
      (for _array_element (Components|GetChildrenComponents (Variables|Default|GetSpawnLocations) false)
        (Utilities|Array|Add (Variables|Default|GetSpawnPoints) (Transformation|GetWorldTransform _array_element)))
      (else
        (Development|PrintString "BP_LevelSpawns: No Spawn Positions" true true "(R=1.000000,G=0.005000,B=0.000000,A=1.000000)" 1e+01)
        (Variables|Default|SetIsDisabled true)))
    (else
      (Development|PrintString "BP_LevelSpawns: No Enemies in the list" true true "(R=1.000000,G=0.005000,B=0.000000,A=1.000000)" 1e+01)
      (Variables|Default|SetIsDisabled true))))

(fn ConstructionScript)