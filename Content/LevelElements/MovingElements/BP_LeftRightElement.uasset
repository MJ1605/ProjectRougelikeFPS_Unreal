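; Moving level element whose cube slides back and forth along the world Y axis.
; Each tick offsets the cube by MoveSpeed scaled by delta time, in the direction given by StartLeft, without sweep.
; StartLeft flips when the projected Y offset from the stationary scene root reaches UpperLimit or LowerLimit.
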(event EventTick
  (params (DeltaSeconds :type Float%20%28single-precision%29))
  (bind _returnvalue (* DeltaSeconds -1.0))
  (bind _cube (Variables|Default|GetCube))
  (bind _defaultsceneroot (Variables|Default|GetDefaultSceneRoot))
  (bind _movespeed (Variables|Default|GetMoveSpeed))
  (bind _movespeed_2 (Variables|Default|GetMoveSpeed))
  (bind _cube_2 (Variables|Default|GetCube))
  (bind _returnvalue_2 (Transformation|GetWorldLocation _cube))
  (bind _returnvalue_3 (Transformation|GetWorldLocation _cube_2))
  (bind _returnvalue_4 (Transformation|GetWorldLocation _defaultsceneroot))
  (bind _returnvalue_5 (* _movespeed DeltaSeconds))
  (bind _returnvalue_6 (* _returnvalue _movespeed_2))
  (bind _returnvalue_7 (Math|Vector|MakeVector 0.0 _returnvalue_5 0.0))
  (bind _y (Math|Vector|BreakVector _returnvalue_4))
  (bind _returnvalue_8 (Math|Vector|MakeVector 0.0 _returnvalue_6 0.0))
  (bind _returnvalue_9 (+ _returnvalue_7 _returnvalue_2))
  (bind _returnvalue_10 (+ _returnvalue_8 _returnvalue_3))
  (if (Variables|Default|GetStart%20Left)
    (Transformation|SetWorldLocation (Variables|Default|GetCube) _returnvalue_9 false false)
    (if (>= (- (.Y (Math|Vector|BreakVector _returnvalue_9)) _y) (Variables|Default|GetUpperLimit))
      (Variables|Default|SetStart%20Left (not (Variables|Default|GetStart%20Left)) :!label _label))
    (else
      (Transformation|SetWorldLocation (Variables|Default|GetCube) _returnvalue_10 false false)
      (if (<= (- (.Y (Math|Vector|BreakVector _returnvalue_10)) _y) (Variables|Default|GetLowerLimit))
        (goto _label)))))

(fn ConstructionScript)