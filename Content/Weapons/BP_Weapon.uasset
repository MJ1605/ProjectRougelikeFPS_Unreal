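; Weapon Blueprint whose only logic is a helper that returns a random direction within a cone, with empty events and construction script.
; GenerateRandomDirectionCone picks a random angle and tangent-scaled radius around +Z, normalizes the vector, then rotates it.
; The 0 to 2π angle feeds degree-based Cosd/Sind, so it spans only about 6 degrees of azimuth.
; Direction's components are used directly as roll, pitch and yaw angles.
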(event EventBeginPlay)

(event Collision|EventActorBeginOverlap
  (params (OtherActor :type Actor%20Object%20Reference)))

(event EventTick
  (params (DeltaSeconds :type Float%20%28single-precision%29)))

(fn ConstructionScript)

(fn GenerateRandomDirectionCone
  (params (Direction :type Vector) (ConeAngle :type Float%20%28double-precision%29))
  (bind (_x _y _z) (Math|Vector|BreakVector Direction))
  (LocalVariables|SetRandomAngle (Math|Random|RandomFloatinRange 0.0 (* (Math|Trig|GetPI) 2.0)))
  (LocalVariables|SetRandomRadius (Math|Random|RandomFloatinRange 0.0 (Math|Trig|Tan(Degrees) (* ConeAngle 0.5))))
  (bind _output_get (LocalVariables|SetRandomDirection (Math|Vector|Normalize (Math|Vector|MakeVector (* (Math|Trig|Cos(Degrees) (LocalVariables|GetRandomAngle)) (LocalVariables|GetRandomRadius)) (* (Math|Trig|Sin(Degrees) (LocalVariables|GetRandomAngle)) (LocalVariables|GetRandomRadius)) 1.0))))
  (bind _output_get_2 (LocalVariables|SetRandomDirection (Math|Vector|RotateVector _output_get (Math|Rotator|MakeRotator _x _y _z))))
  (return _output_get_2))