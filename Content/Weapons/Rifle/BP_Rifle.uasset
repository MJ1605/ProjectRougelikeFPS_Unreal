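; BP_Rifle is a rifle weapon actor that fires bullet projectiles at a limited fire rate.
; Fire spawns a BP_RifleBullet at the BulletSpawn transform, passes it speed and damage, then starts a cooldown from Firerate.
; Tick counts the cooldown down through ProcessFiredt, clamping it to zero so the next shot is allowed.
; On BeginPlay the root component is shifted by an Offset transform.
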(event EventTick
  (params (DeltaSeconds :type Float%20%28single-precision%29))
  (CallFunction|ProcessFiredt DeltaSeconds))

(event EventBeginPlay
  (Class|SceneComponent|AddWorldTransform (Variables|Default|GetDefaultSceneRoot) (Variables|Default|GetOffset) false false))

(event EventFire
  (if (== (Variables|Default|GetFiredt) 0.0)
    (bind _returnvalue (Game|SpawnActorfromClass "/Game/Weapons/Rifle/BP_RifleBullet.BP_RifleBullet_C" (Transformation|GetWorldTransform (Variables|Default|GetBulletSpawn)) "Undefined" 0 0))
    (Default|InitValues _returnvalue (Variables|Default|GetBullet%20Speed) (Variables|Default|GetWeapon%20Damage))
    (Variables|Default|SetFiredt (Variables|Default|GetFirerate))))

(fn ConstructionScript)

(fn ProcessFiredt
  (params (ElaspedTime :type Float%20%28double-precision%29))
  (if (not (<= (Variables|Default|GetFiredt) 0.0))
    (if (< (- (Variables|Default|GetFiredt) ElaspedTime) 0.0)
      (Variables|Default|SetFiredt 0.0)
      (else
        (Variables|Default|SetFiredt (- (Variables|Default|GetFiredt) ElaspedTime))))))