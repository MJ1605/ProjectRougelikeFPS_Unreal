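; BP_RifleBullet is a rifle projectile that damages whatever it hits and then destroys itself.
; InitValues sets the projectile movement's initial and max speed and stores a damage value in ProjectileDamage.
; The hit event applies a hardcoded damage amount, not ProjectileDamage, crediting player controller 0 as instigator.
; Tick counts FLifetime down and destroys the bullet when it runs out.
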(event Collision|EventHit
  (params (MyComp :type Primitive%20Component%20Object%20Reference) (Other :type Actor%20Object%20Reference) (OtherComp :type Primitive%20Component%20Object%20Reference) (bSelfMoved :type Boolean) (HitLocation :type Vector :default "0, 0, 0") (HitNormal :type Vector :default "0, 0, 0") (NormalImpulse :type Vector :default "0, 0, 0") (Hit :type Hit%20Result%20Structure%20%28by%20ref%29))
  (Game|Damage|ApplyDamage Other 1e+01 (Game|GetPlayerController 0) self)
  (Actor|DestroyActor))

(event EventTick
  (params (DeltaSeconds :type Float%20%28single-precision%29))
  ;[1 1 1] Process the lifetime
  (bind _output_get (Variables|Default|SetfLifetime (- (Variables|Default|GetfLifetime) DeltaSeconds)))
  (if (<= _output_get 0.0)
    (Actor|DestroyActor)))

(fn ConstructionScript)

(fn InitValues
  (params (Velocity :type Float%20%28double-precision%29) (Damage :type Float%20%28double-precision%29))
  (bind _projectilemovement (Variables|Default|GetProjectileMovement))
  (bind _output_get (Variables|/Script/Engine.ProjectileMovementComponent|SetInitialSpeed _projectilemovement Velocity))
  (Variables|/Script/Engine.ProjectileMovementComponent|SetMaxSpeed _projectilemovement _output_get)
  (Variables|Default|SetProjectile%20Damage Damage))