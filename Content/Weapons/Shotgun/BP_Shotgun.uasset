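; Shotgun weapon Blueprint that fires a BP_RifleBullet with random spread.
; On BeginPlay it applies an Offset world transform to its root component.
; Each Fire event spawns one bullet at BulletSpawn, with player pawn 0 as instigator.
; Its direction is randomized in a SpreadAngle cone around the Cube's forward vector, then further rotated by BulletSpawn's world rotation.
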(event EventFire
  (bind _bulletspawn (Variables|Default|GetBulletSpawn))
  (bind _returnvalue (Transformation|GetWorldTransform _bulletspawn))
  (bind (_location _rotation _scale) (Math|Transform|BreakTransform _returnvalue))
  (bind _randomdir (CallFunction|GenerateRandomDirectionCone (Math|Vector|GetForwardVector (Variables|Default|GetCube)) (Variables|Default|GetSpreadAngle)))
  (Game|SpawnActorfromClass "/Game/Weapons/Rifle/BP_RifleBullet.BP_RifleBullet_C" (Math|Transform|MakeTransform _location (Math|Rotator|MakeRotfromX (Math|Vector|RotateVector _randomdir _rotation)) _scale) "Undefined" 0 (Game|Player|GetPlayerPawn 0)))

(event EventBeginPlay
  (Class|SceneComponent|AddWorldTransform (Variables|Default|GetDefaultSceneRoot) (Variables|Default|GetOffset) false false))

(fn ConstructionScript
  (|CallParentFunction))