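; BP_ShotgunBullet is a shotgun projectile actor that damages whatever it hits.
; InitValues sets the projectile movement's initial and max speed from one velocity value and stores the damage.
; BeginPlay scales the Cube from ProjectileTransform, and Tick counts Lifetime down to destroy the actor on expiry.
; A Hit applies normal-type damage to the other actor, then destroys the bullet.
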(event EventBeginPlay
  ;[1 1 1] Set the size of the cube at the start
  (Transformation|SetWorldScale3D (Variables|Default|GetCube) (.Scale (Math|Transform|BreakTransform (Variables|Default|GetProjectileTransform)))))

(event EventTick
  (params (DeltaSeconds :type Float%20%28single-precision%29))
  ;[1 1 1] Destroy when lifetime is over
  (bind _output_get (Variables|Default|SetLifetime (- (Variables|Default|GetLifetime) DeltaSeconds)))
  (if (<= _output_get 0.0)
    (Actor|DestroyActor)))

(event Collision|EventHit
  (params (MyComp :type Primitive%20Component%20Object%20Reference) (Other :type Actor%20Object%20Reference) (OtherComp :type Primitive%20Component%20Object%20Reference) (bSelfMoved :type Boolean) (HitLocation :type Vector :default "0, 0, 0") (HitNormal :type Vector :default "0, 0, 0") (NormalImpulse :type Vector :default "0, 0, 0") (Hit :type Hit%20Result%20Structure%20%28by%20ref%29))
  ;[1 1 1] Handle Hit
  (Game|Damage|ApplyDamage Other (Variables|Default|GetProjectDamage) 0 self "/Game/Weapons/DamageTypes/DamageType_Normal.DamageType_Normal_C")
  (Actor|DestroyActor))

(fn ConstructionScript)

(fn InitValues
  (params (Velocity :type Float%20%28double-precision%29) (Damage :type Float%20%28double-precision%29))
  (bind _projectilemovement (Variables|Default|GetProjectileMovement))
  (bind _output_get (Variables|/Script/Engine.ProjectileMovementComponent|SetInitialSpeed _projectilemovement Velocity))
  (Variables|/Script/Engine.ProjectileMovementComponent|SetMaxSpeed _projectilemovement _output_get)
  (Variables|Default|SetProjectDamage Damage))